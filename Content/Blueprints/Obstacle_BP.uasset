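; Obstacle for the GravityCube game that moves upward and ends the game when the player's cube touches it.
; The construction script creates a dynamic material on the Cube, and BeginPlay gives it a random glow color.
; Tick raises the Cube in world Z at a constant, delta-time-scaled speed.
; Overlap with a GravityCube_BP calls GameOver on the GravityCube game mode.
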(event OnComponentBeginOverlap(Cube)
  (params (OverlappedComponent :type Primitive%20Component%20Object%20Reference) (OtherActor :type Actor%20Object%20Reference) (OtherComp :type Primitive%20Component%20Object%20Reference) (OtherBodyIndex :type Integer) (bFromSweep :type Boolean) (SweepResult :type Hit%20Result%20Structure%20%28by%20ref%29))
  (Utilities|Casting|CastToGravityCube_BP OtherActor)
  (bind _asgravity_cube_game_mode (Utilities|Casting|CastToGravityCube_GameMode (Game|GetGameMode)))
  (Default|GameOver _asgravity_cube_game_mode))

(event EventBeginPlay
  ;[1 1 1] Random Glow Color
  (Rendering|Material|SetVectorParameterValue (Variables|Default|GetDynamicMaterial) "Color" (Utilities|Struct|MakeLinearColor (Math|Random|RandomFloatinRange 0.0 1.0) (Math|Random|RandomFloatinRange 0.0 1.0) (Math|Random|RandomFloatinRange 0.0 1.0) 1.0) :!class /Script/Engine.MaterialInstanceDynamic))

(event EventTick
  (params (DeltaSeconds :type Float%20%28single-precision%29))
  (bind _cube (Variables|Default|GetCube))
  (bind _returnvalue (Transformation|GetWorldLocation _cube))
  (Transformation|SetWorldLocation (Variables|Default|GetCube) (Math|Vector|MakeVector (.x _returnvalue) (.y _returnvalue) (+ (.z _returnvalue) (* 2.7e+03 (Utilities|Time|GetWorldDeltaSeconds)))) false false))

(fn ConstructionScript
  (bind _returnvalue (Rendering|Material|CreateDynamicMaterialInstance (Variables|Default|GetCube) 0 0 :!class /Script/Engine.PrimitiveComponent))
  (Variables|Default|SetDynamicMaterial _returnvalue))