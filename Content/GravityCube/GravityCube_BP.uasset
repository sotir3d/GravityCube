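; Player-controlled cube that slides along four walls and flips gravity to cross to the opposite one.
; Tick checks axis input against tilt thresholds for a push away from the current wall, then applies forced movement along a gravity vector.
; Cube hits stop the flip and set the wall state by matching the hit actor's object name.
; Axis events move the cube along its wall or sideways mid-flip, depending on that state.
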(event OnComponentHit(Cube)
  (params (HitComponent :type Primitive%20Component%20Object%20Reference) (OtherActor :type Actor%20Object%20Reference) (OtherComp :type Primitive%20Component%20Object%20Reference) (NormalImpulse :type Vector :default "0, 0, 0") (Hit :type Hit%20Result%20Structure%20%28by%20ref%29))
  (CallFunction|SetCurrentWall OtherActor)
  (Variables|Default|SetIsFlippingGravity false))

(event EventBeginPlay
  (Transformation|SetWorldLocation (Variables|Default|GetCube) "-430.000000,0.000000,115.000000" false false))

(event EventTick
  (params (DeltaSeconds :type Float%20%28single-precision%29))
  (CallFunction|DirectionHandler)
  (if (Variables|Default|GetIsFlippingGravity)
    (Pawn|Input|AddMovementInput (Variables|Default|GetGravityVector) 1.0 true)))

(event Input|AxisEvents|InputAxisMoveUpDown
  (params (AxisValue :type Float%20%28single-precision%29))
  (CallFunction|ControlSideWalls))

(event Input|AxisEvents|InputAxisMoveLeftRight
  (params (AxisValue :type Float%20%28single-precision%29))
  (CallFunction|ControlTopBottomWalls))

(fn ConstructionScript)

(fn SetCurrentWall
  (params (InActor :type Actor%20Object%20Reference))
  (bind _returnvalue (Utilities|GetObjectName InActor))
  (if (or (Utilities|Enum|Equal(Enum) (Variables|Default|GetCurrentState) "NewEnumerator4") (Utilities|Enum|Equal(Enum) (Variables|Default|GetCurrentState) "NewEnumerator5"))
    (if (Utilities|Enum|Equal(Enum) _returnvalue "BottomWall")
      (Variables|Default|SetCurrentState "NewEnumerator3")
      (elif (Utilities|Enum|Equal(Enum) _returnvalue "RightWall")
        (Variables|Default|SetCurrentState "NewEnumerator1")
        (elif (Utilities|Enum|Equal(Enum) _returnvalue "TopWall")
          (Variables|Default|SetCurrentState "NewEnumerator2")
          (elif (Utilities|Enum|Equal(Enum) _returnvalue "LeftWall")
            (Variables|Default|SetCurrentState "NewEnumerator0")))))))

(fn ControlTopBottomWalls
  (bind _returnvalue (Input|AxisValues|GetMoveLeftRight))
  (bind _returnvalue_2 (Input|AxisValues|GetMoveLeftRight))
  (bind _currentstate (Variables|Default|GetCurrentState))
  (bind _tiltdegree (Variables|Default|GetTiltDegree))
  (if (Math|Boolean|ORBoolean (Utilities|Enum|Equal(Enum) _currentstate "NewEnumerator3") (Utilities|Enum|Equal(Enum) _currentstate "NewEnumerator2") (Utilities|Enum|Equal(Enum) _currentstate "NewEnumerator4"))
    (if (> _returnvalue_2 _tiltdegree)
      (Pawn|Input|AddMovementInput (Math|Vector|MakeVector 0.0 1.0 0.0) 1.0 false)
      (elif (< _returnvalue_2 (* _tiltdegree -1.0))
        (Pawn|Input|AddMovementInput (Math|Vector|MakeVector 0.0 -1.0 0.0) 1.0 false)
        (elif (> _returnvalue 0.05)
          (Pawn|Input|AddMovementInput (Math|Vector|MakeVector 0.0 1.0 0.0) 0.8 false)
          (elif (< _returnvalue -0.05)
            (Pawn|Input|AddMovementInput (Math|Vector|MakeVector 0.0 -1.0 0.0) 0.8 false)))))))

(fn DirectionHandler
  (bind _returnvalue (Input|AxisValues|GetMoveUpDown))
  (bind _returnvalue_2 (Input|AxisValues|GetMoveUpDown))
  (if (and (or (Utilities|Enum|Equal(Enum) (Variables|Default|GetCurrentState) "NewEnumerator3") false) (or (== _returnvalue 1.0) (> _returnvalue (Variables|Default|GetGravityDegree))))
    (Variables|Default|SetIsFlippingGravity true)
    (Variables|Default|SetGravityVector (Math|Vector|MakeVector 1.0 0.0 0.0))
    (Variables|Default|SetCurrentState "NewEnumerator4" :!label _label)
    (elif (and (or (Utilities|Enum|Equal(Enum) (Variables|Default|GetCurrentState) "NewEnumerator2") false) (or (== _returnvalue_2 -1.0) (< _returnvalue_2 (* (Variables|Default|GetGravityDegree) -1.0))))
      (Variables|Default|SetIsFlippingGravity true)
      (Variables|Default|SetGravityVector (Math|Vector|MakeVector -1.0 0.0 0.0))
      (goto _label)
      (else
        (if (and (or (Utilities|Enum|Equal(Enum) (Variables|Default|GetCurrentState) "NewEnumerator0") false) (> (Input|AxisValues|GetMoveLeftRight) (Variables|Default|GetTiltDegree)))
          (Variables|Default|SetIsFlippingGravity true)
          (Variables|Default|SetGravityVector (Math|Vector|MakeVector 0.0 1.0 0.0))
          (elif (and (or (Utilities|Enum|Equal(Enum) (Variables|Default|GetCurrentState) "NewEnumerator1") false) (< (Input|AxisValues|GetMoveLeftRight) (* (Variables|Default|GetTiltDegree) -1.0)))
            (Variables|Default|SetIsFlippingGravity true)
            (Variables|Default|SetGravityVector (Math|Vector|MakeVector 0.0 -1.0 0.0))
            (else
              (return))))
        (Variables|Default|SetCurrentState "NewEnumerator5"))))
  (return))

(fn ControlSideWalls
  (bind _returnvalue (Input|AxisValues|GetMoveUpDown))
  (bind _currentstate (Variables|Default|GetCurrentState))
  (if (Math|Boolean|ORBoolean (Utilities|Enum|Equal(Enum) _currentstate "NewEnumerator0") (Utilities|Enum|Equal(Enum) _currentstate "NewEnumerator1") (Utilities|Enum|Equal(Enum) _currentstate "NewEnumerator5"))
    (if (or (> _returnvalue (Variables|Default|GetGravityDegree)) (== _returnvalue 1.0))
      (Pawn|Input|AddMovementInput (Math|Vector|MakeVector 1.0 0.0 0.0) 1.0 false)
      (elif (or (< _returnvalue (* (Variables|Default|GetGravityDegree) -1.0)) (== _returnvalue -1.0))
        (Pawn|Input|AddMovementInput (Math|Vector|MakeVector -1.0 0.0 0.0) 1.0 false)))))